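; StartTile is a runner-game track tile with a SpawnObstacles function for populating its three lanes, though nothing in this graph calls it.
; Each lane runs its own fallthrough chain of range checks, spawning at most one pipe, box, bonus point, magnet or boots actor at the lane component's transform.
; Every random roll has a zero-to-zero range, so outcomes never vary as configured here.
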(fn `Spawn Obstacles`
  (bind _returnvalue (`KismetMathLibrary.RandomFloatInRange` 0.0))
  (bind _returnvalue_2 (`KismetMathLibrary.RandomFloatInRange` 0.0))
  (bind _returnvalue_3 (`KismetMathLibrary.RandomFloatInRange` 0.0))
  (bind _returnvalue_4 (`SceneComponent.K2_GetComponentToWorld` (`self.Lane0`)))
  (bind _returnvalue_5 (`SceneComponent.K2_GetComponentToWorld` (`self.Lane1`)))
  (bind _returnvalue_6 (`SceneComponent.K2_GetComponentToWorld` (`self.Lane2`)))
  (if (`KismetMathLibrary.InRange_FloatFloat` _returnvalue 0.0 1.0 true false)
    (`|SpawnActorFromClass` "/Game/RunnerFiles/Blueprints/PipeObstacle.PipeObstacle_C" _returnvalue_4 "Undefined" "OverrideRootScale" null null)
    (elif (`KismetMathLibrary.InRange_FloatFloat` _returnvalue 0.0 1.0 true false)
      (`|SpawnActorFromClass` "/Game/RunnerFiles/Blueprints/BoxObstacle.BoxObstacle_C" _returnvalue_4 "Undefined" "OverrideRootScale" null null)
      (elif (`KismetMathLibrary.InRange_FloatFloat` _returnvalue 0.0 1.0 true false)
        (`|SpawnActorFromClass` "/Game/RunnerFiles/Blueprints/BonusPoint_Pickup.BonusPoint_Pickup_C" _returnvalue_4 "Undefined" "OverrideRootScale" null null)
        (elif (`KismetMathLibrary.InRange_FloatFloat` _returnvalue 0.0 1.0 true false)
          (`|SpawnActorFromClass` "/Game/RunnerFiles/Blueprints/Magnet_Pickup.Magnet_Pickup_C" _returnvalue_4 "Undefined" "OverrideRootScale" null null)
          (elif (`KismetMathLibrary.InRange_FloatFloat` _returnvalue 0.0 1.0 true false)
            (`|SpawnActorFromClass` "/Game/RunnerFiles/Blueprints/Boots_Pickup.Boots_Pickup_C" _returnvalue_4 "Undefined" "OverrideRootScale" null null))))))
  (if (`KismetMathLibrary.InRange_FloatFloat` _returnvalue_2 0.0 1.0 true false)
    (`|SpawnActorFromClass` "/Game/RunnerFiles/Blueprints/PipeObstacle.PipeObstacle_C" _returnvalue_5 "Undefined" "OverrideRootScale" null null)
    (elif (`KismetMathLibrary.InRange_FloatFloat` _returnvalue_2 0.0 1.0 true false)
      (`|SpawnActorFromClass` "/Game/RunnerFiles/Blueprints/BoxObstacle.BoxObstacle_C" _returnvalue_5 "Undefined" "OverrideRootScale" null null)
      (elif (`KismetMathLibrary.InRange_FloatFloat` _returnvalue_2 0.0 1.0 true false)
        (`|SpawnActorFromClass` "/Game/RunnerFiles/Blueprints/BonusPoint_Pickup.BonusPoint_Pickup_C" _returnvalue_5 "Undefined" "OverrideRootScale" null null)
        (elif (`KismetMathLibrary.InRange_FloatFloat` _returnvalue_2 0.0 1.0 true false)
          (`|SpawnActorFromClass` "/Game/RunnerFiles/Blueprints/Magnet_Pickup.Magnet_Pickup_C" _returnvalue_5 "Undefined" "OverrideRootScale" null null)
          (elif (`KismetMathLibrary.InRange_FloatFloat` _returnvalue_2 0.0 1.0 true false)
            (`|SpawnActorFromClass` "/Game/RunnerFiles/Blueprints/Boots_Pickup.Boots_Pickup_C" _returnvalue_5 "Undefined" "OverrideRootScale" null null))))))
  (if (`KismetMathLibrary.InRange_FloatFloat` _returnvalue_3 0.0 1.0 true false)
    (`|SpawnActorFromClass` "/Game/RunnerFiles/Blueprints/PipeObstacle.PipeObstacle_C" _returnvalue_6 "Undefined" "OverrideRootScale" null null)
    (elif (`KismetMathLibrary.InRange_FloatFloat` _returnvalue_3 0.0 1.0 true false)
      (`|SpawnActorFromClass` "/Game/RunnerFiles/Blueprints/BoxObstacle.BoxObstacle_C" _returnvalue_6 "Undefined" "OverrideRootScale" null null)
      (elif (`KismetMathLibrary.InRange_FloatFloat` _returnvalue_3 0.0 1.0 true false)
        (`|SpawnActorFromClass` "/Game/RunnerFiles/Blueprints/BonusPoint_Pickup.BonusPoint_Pickup_C" _returnvalue_6 "Undefined" "OverrideRootScale" null null)
        (elif (`KismetMathLibrary.InRange_FloatFloat` _returnvalue_3 0.0 1.0 true false)
          (`|SpawnActorFromClass` "/Game/RunnerFiles/Blueprints/Magnet_Pickup.Magnet_Pickup_C" _returnvalue_6 "Undefined" "OverrideRootScale" null null)
          (elif (`KismetMathLibrary.InRange_FloatFloat` _returnvalue_3 0.0 1.0 true false)
            (`|SpawnActorFromClass` "/Game/RunnerFiles/Blueprints/Boots_Pickup.Boots_Pickup_C" _returnvalue_6 "Undefined" "OverrideRootScale" null null)))))))

(fn `UserConstructionScript`)