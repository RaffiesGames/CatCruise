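; Boots_Pickup is a runner-game pickup that temporarily activates the player character's jump power-up through the JumpActive flag.
; When a ThirdPersonCharacter overlaps it, it plays a sound, shows a Boots_Duration widget, sets the flag and hides its mesh.
; A five-second retriggerable delay then clears the flag on player character 0.
; The actor is never destroyed or its collision disabled, so further overlaps can retrigger the effect.
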(event `self.ReceiveActorBeginOverlap`
  (params (OtherActor :type "Actor Object Reference"))
  (bind _asthird_person_character (cast `/Game/RunnerFiles/Blueprints/ThirdPersonCharacter` OtherActor))
  (`GameplayStatics.PlaySound2D` "/Game/RunnerFiles/SFX/Pickup_SFX_Cue.Pickup_SFX_Cue" 1.0 1.0 0.0 null null)
  (bind _returnvalue (`|CreateWidget` "/Game/RunnerFiles/Blueprints/Widgets/Boots_Duration.Boots_Duration_C" (`GameplayStatics.GetPlayerController` 0)))
  (`UserWidget.AddToViewport` _returnvalue 4)
  (set `/Game/RunnerFiles/Blueprints/ThirdPersonCharacter.JumpActive` true _asthird_person_character)
  (`SceneComponent.SetVisibility` (`self.StaticMesh`) false false)
  (`KismetSystemLibrary.RetriggerableDelay` 5.0)
  (bind _asthird_person_character_2 (cast `/Game/RunnerFiles/Blueprints/ThirdPersonCharacter` (`GameplayStatics.GetPlayerCharacter` 0)))
  (set `/Game/RunnerFiles/Blueprints/ThirdPersonCharacter.JumpActive` false _asthird_person_character_2))

(fn `UserConstructionScript`)