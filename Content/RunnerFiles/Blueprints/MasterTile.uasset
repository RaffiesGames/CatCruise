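; MasterTile is an endless-runner track tile that populates three lanes and advances the run when crossed.
; On BeginPlay, chained random range rolls pick a pipe, box, bonus, magnet or boots per lane, withholding powerups already active.
; A box in Lane0 skips Lane1's roll.
; Player overlap with its trigger has the GameMode spawn another tile, adds multiplied score, raises clamped walk speed, then destroys the tile after a delay.
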(event `self.ReceiveBeginPlay`
  (`self.Spawn Obstacles`))

(event `self.Box.OnComponentBeginOverlap`
  (params (OverlappedComponent :type "PrimitiveComponent Object Reference") (OtherActor :type "Actor Object Reference") (OtherComp :type "PrimitiveComponent Object Reference") (OtherBodyIndex :type Integer) (bFromSweep :type Boolean) (SweepResult :type "HitResult Structure (by ref)"))
  (cast `/Game/RunnerFiles/Blueprints/ThirdPersonCharacter` OtherActor)
  (bind _asthird_person_game_mode (cast `/Game/ThirdPersonBP/Blueprints/ThirdPersonGameMode` (`GameplayStatics.GetGameMode`)))
  (`/Game/ThirdPersonBP/Blueprints/ThirdPersonGameMode.SpawnTile` _asthird_person_game_mode)
  (bind _asthird_person_game_mode_2 (cast `/Game/ThirdPersonBP/Blueprints/ThirdPersonGameMode` (`GameplayStatics.GetGameMode`)))
  (set `/Game/ThirdPersonBP/Blueprints/ThirdPersonGameMode.CurrentScore` (+ (`/Game/ThirdPersonBP/Blueprints/ThirdPersonGameMode.CurrentScore` _asthird_person_game_mode_2) (* 1 (`/Game/ThirdPersonBP/Blueprints/ThirdPersonGameMode.ScoreMultiplier` _asthird_person_game_mode_2))) _asthird_person_game_mode_2)
  (bind _ascharacter (cast `Character` (`GameplayStatics.GetPlayerCharacter` 0)))
  (bind _charactermovement (`Character.CharacterMovement` _ascharacter))
  (set `CharacterMovementComponent.MaxWalkSpeed` (`KismetMathLibrary.FClamp` (* (`CharacterMovementComponent.MaxWalkSpeed` _charactermovement) 1.02) 1500.0 3500.0) _charactermovement)
  (`KismetSystemLibrary.Delay` 2.0)
  (`self.K2_DestroyActor`))

(fn `CheckJump`
  (returns (NewParam :type Boolean))
  (bind _asthird_person_character (cast `/Game/RunnerFiles/Blueprints/ThirdPersonCharacter` (`GameplayStatics.GetPlayerCharacter` 0)))
  (return (`/Game/RunnerFiles/Blueprints/ThirdPersonCharacter.JumpActive` _asthird_person_character)))

(fn `CheckMagnet`
  (returns (NewParam :type Boolean))
  (bind _asthird_person_character (cast `/Game/RunnerFiles/Blueprints/ThirdPersonCharacter` (`GameplayStatics.GetPlayerCharacter` 0)))
  (return (`/Game/RunnerFiles/Blueprints/ThirdPersonCharacter.MagnetActive` _asthird_person_character)))

(fn `Spawn Obstacles`
  (bind _returnvalue (`SceneComponent.K2_GetComponentToWorld` (`self.Lane0`)))
  (bind _returnvalue_2 (`KismetMathLibrary.RandomFloatInRange` (`self.RandomMin`) (`self.RandomMax`)))
  (bind _returnvalue_3 (`SceneComponent.K2_GetComponentToWorld` (`self.Lane1`)))
  (bind _returnvalue_4 (`SceneComponent.K2_GetComponentToWorld` (`self.Lane2`)))
  (bind _returnvalue_5 (`KismetMathLibrary.RandomFloatInRange` (`self.RandomMin`) (`self.RandomMax`)))
  (bind _returnvalue_6 (`KismetMathLibrary.RandomFloatInRange` (`self.RandomMin`) (`self.RandomMax`)))
  (if (`KismetMathLibrary.InRange_FloatFloat` _returnvalue_2 (`self.PipeMin`) (`self.PipeMax`) true false)
    (`|SpawnActorFromClass` "/Game/RunnerFiles/Blueprints/PipeObstacle.PipeObstacle_C" _returnvalue "Undefined" "OverrideRootScale" null null)
    (if (`KismetMathLibrary.InRange_FloatFloat` _returnvalue_5 (`self.PipeMin`) (`self.PipeMax`) true false) :!label _label
      (`|SpawnActorFromClass` "/Game/RunnerFiles/Blueprints/PipeObstacle.PipeObstacle_C" _returnvalue_3 "Undefined" "OverrideRootScale" null null)
      (elif (`KismetMathLibrary.InRange_FloatFloat` _returnvalue_5 (`self.BoxMin`) (`self.BoxMax`) true false)
        (`|SpawnActorFromClass` "/Game/RunnerFiles/Blueprints/BoxObstacle.BoxObstacle_C" _returnvalue_3 "Undefined" "OverrideRootScale" null null)
        (elif (`KismetMathLibrary.InRange_FloatFloat` _returnvalue_5 (`self.DonutMin`) (`self.DonutMax`) true false)
          (`|SpawnActorFromClass` "/Game/RunnerFiles/Blueprints/BonusPoint_Pickup.BonusPoint_Pickup_C" _returnvalue_3 "Undefined" "OverrideRootScale" null null)
          (else
            (bind _newparam (`self.CheckMagnet`))
            (if _newparam
              (bind _newparam_2 (`self.CheckJump` :!label _label_2))
              (if _newparam_2
                _
                (elif (`KismetMathLibrary.InRange_FloatFloat` _returnvalue_5 (`self.JumpMin`) (`self.JumpMax`) true false)
                  (`|SpawnActorFromClass` "/Game/RunnerFiles/Blueprints/Boots_Pickup.Boots_Pickup_C" _returnvalue_3 "Undefined" "OverrideRootScale" null null)))
              (elif (`KismetMathLibrary.InRange_FloatFloat` _returnvalue_5 (`self.MagnetMin`) (`self.MagnetMax`) true false)
                (`|SpawnActorFromClass` "/Game/RunnerFiles/Blueprints/Magnet_Pickup.Magnet_Pickup_C" _returnvalue_3 "Undefined" "OverrideRootScale" null null)
                (else
                  (goto _label_2))))))))
    (elif (`KismetMathLibrary.InRange_FloatFloat` _returnvalue_2 (`self.BoxMin`) (`self.BoxMax`) true false)
      (`|SpawnActorFromClass` "/Game/RunnerFiles/Blueprints/BoxObstacle.BoxObstacle_C" _returnvalue "Undefined" "OverrideRootScale" null null)
      (elif (`KismetMathLibrary.InRange_FloatFloat` _returnvalue_2 (`self.DonutMin`) (`self.DonutMax`) true false)
        (`|SpawnActorFromClass` "/Game/RunnerFiles/Blueprints/BonusPoint_Pickup.BonusPoint_Pickup_C" _returnvalue "Undefined" "OverrideRootScale" null null)
        (goto _label)
        (else
          (bind _newparam_3 (`self.CheckMagnet`))
          (if _newparam_3
            _
            (elif (`KismetMathLibrary.InRange_FloatFloat` _returnvalue_2 (`self.MagnetMin`) (`self.MagnetMax`) true false)
              (`|SpawnActorFromClass` "/Game/RunnerFiles/Blueprints/Magnet_Pickup.Magnet_Pickup_C" _returnvalue "Undefined" "OverrideRootScale" null null)
              (goto _label)
              (else
                _)))
          (bind _newparam_4 (`self.CheckJump`))
          (if _newparam_4
            (goto _label)
            (elif (`KismetMathLibrary.InRange_FloatFloat` _returnvalue_2 (`self.JumpMin`) (`self.JumpMax`) true false)
              (`|SpawnActorFromClass` "/Game/RunnerFiles/Blueprints/Boots_Pickup.Boots_Pickup_C" _returnvalue "Undefined" "OverrideRootScale" null null)
              (goto _label)
              (else
                (goto _label))))))))
  (if (`KismetMathLibrary.InRange_FloatFloat` _returnvalue_6 (`self.PipeMin`) (`self.PipeMax`) true false)
    (`|SpawnActorFromClass` "/Game/RunnerFiles/Blueprints/PipeObstacle.PipeObstacle_C" _returnvalue_4 "Undefined" "OverrideRootScale" null null)
    (elif (`KismetMathLibrary.InRange_FloatFloat` _returnvalue_6 (`self.BoxMin`) (`self.BoxMax`) true false)
      (`|SpawnActorFromClass` "/Game/RunnerFiles/Blueprints/BoxObstacle.BoxObstacle_C" _returnvalue_4 "Undefined" "OverrideRootScale" null null)
      (elif (`KismetMathLibrary.InRange_FloatFloat` _returnvalue_6 (`self.DonutMin`) (`self.DonutMax`) true false)
        (`|SpawnActorFromClass` "/Game/RunnerFiles/Blueprints/BonusPoint_Pickup.BonusPoint_Pickup_C" _returnvalue_4 "Undefined" "OverrideRootScale" null null)
        (else
          (bind _newparam_5 (`self.CheckMagnet`))
          (if _newparam_5
            (bind _newparam_6 (`self.CheckJump` :!label _label_3))
            (if _newparam_6
              _
              (elif (`KismetMathLibrary.InRange_FloatFloat` _returnvalue_6 (`self.JumpMin`) (`self.JumpMax`) true false)
                (`|SpawnActorFromClass` "/Game/RunnerFiles/Blueprints/Boots_Pickup.Boots_Pickup_C" _returnvalue_4 "Undefined" "OverrideRootScale" null null)))
            (elif (`KismetMathLibrary.InRange_FloatFloat` _returnvalue_6 (`self.MagnetMin`) (`self.MagnetMax`) true false)
              (`|SpawnActorFromClass` "/Game/RunnerFiles/Blueprints/Magnet_Pickup.Magnet_Pickup_C" _returnvalue_4 "Undefined" "OverrideRootScale" null null)
              (else
                (goto _label_3)))))))))

(fn `UserConstructionScript`)